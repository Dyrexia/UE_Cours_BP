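; Door Blueprint that toggles between closed and open by snapping the Door component's relative yaw between 0 and 90 degrees.
; Activate and Deactivate both call ChangeState, which decides from the current yaw, so either event simply flips the door.
; A separate Open event spins the door briefly through RotatingMovement, but ChangeState leaves it unused; Close is empty and the IsOpen toggle logic is disconnected.
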(event Custom|Open
  (bind _rotatingmovement (Variables|Default|GetRotatingMovement))
  (Components|Activation|Activate _rotatingmovement false)
  (Utilities|FlowControl|Delay 1.0)
  (Components|Activation|Deactivate _rotatingmovement))

(event Custom|Close)

(event EventDeactivate
  (CallFunction|ChangeState))

(event EventActivate
  (CallFunction|ChangeState))

(fn ConstructionScript)

(fn ChangeState
  (bind _door (Variables|Default|GetDoor))
  (if (> (.yaw (Variables|/Script/Engine.SceneComponent|GetRelativeRotation _door)) 0.0)
    (Transformation|SetRelativeRotation _door "0.000000,0.000000,0.000000" false false)
    (else
      (Transformation|SetRelativeRotation _door "0.000000,90.000000,0.000000" false false))))