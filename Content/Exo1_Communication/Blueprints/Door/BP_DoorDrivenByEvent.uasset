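; A door actor that opens and closes in response to a switch, part of an exercise on Blueprint communication.
; On BeginPlay it binds its Activate event to the ActivateControlables dispatcher of the referenced BPInterrupteur.
; Each activation calls ChangeState, which instantly snaps the Door component's relative yaw between closed and a quarter turn, using the current rotation as the state.
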(event Custom|Activate
  (CallFunction|ChangeState))

(event EventBeginPlay
  (EventDispatchers|BindEventtoActivateControlables (Variables|Default|GetBP_Interrupteur) (delegate Custom|Activate)))

(fn ConstructionScript)

(fn ChangeState
  (bind _door (Variables|Default|GetDoor))
  (if (> (.yaw (Variables|/Script/Engine.SceneComponent|GetRelativeRotation _door)) 0.0)
    (Transformation|SetRelativeRotation _door "0, 0, 0" false false)
    (else
      (Transformation|SetRelativeRotation _door "0.000000,90.000000,0.000000" false false))))