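; BP_Door is a door Blueprint with an IsOpen state that ChangeState toggles, calling Open or Close.
; Open swings the door by activating its RotatingMovement component, then deactivating it after a one-second Delay, so the travel depends on rotation rate and time.
; Close is an empty event, so toggling back only clears the flag without moving the door.
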(event Custom|Open
  (bind _rotatingmovement (Variables|Default|GetRotatingMovement))
  (Components|Activation|Activate _rotatingmovement false)
  (Utilities|FlowControl|Delay 1.0)
  (Components|Activation|Deactivate _rotatingmovement))

(event Custom|Close)

(fn ConstructionScript)

(fn ChangeState
  (if (Variables|Default|GetIsOpen)
    (Variables|Default|SetIsOpen false)
    (CallFunction|Close)
    (else
      (Variables|Default|SetIsOpen true)
      (CallFunction|Open))))